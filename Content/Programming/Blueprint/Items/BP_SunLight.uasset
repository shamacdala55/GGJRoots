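; BP_SunLight is a pickup that restores one point of life to BP_GGJRootsCharacter when it overlaps the sphere.
; A character at zero life or above MaxLife only gets a life printout, so one exactly at max still gains a point.
; After adding life, it refreshes the life counter through the local player's RootHUD and destroys itself.
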(event OnComponentBeginOverlap(Sphere)
  (params (OverlappedComponent :type Primitive%20Component%20Object%20Reference) (OtherActor :type Actor%20Object%20Reference) (OtherComp :type Primitive%20Component%20Object%20Reference) (OtherBodyIndex :type Integer) (bFromSweep :type Boolean) (SweepResult :type Hit%20Result%20Structure%20%28by%20ref%29))
  (bind _asbp_ggjroots_character (Utilities|Casting|CastToBP_GGJRootsCharacter OtherActor))
  (Utilities|IsValid _asbp_ggjroots_character
    (:Is%20Valid
      (if (== (Variables|/Script/GGJRoots.GGJRootsCharacter|GetCurrentLife _asbp_ggjroots_character) 0)
        (Development|PrintString (Utilities|String|ToString(Integer) (Variables|/Script/GGJRoots.GGJRootsCharacter|GetCurrentLife _asbp_ggjroots_character)) :!label _label)
        (elif (> (stale _output_get) (Variables|/Script/GGJRoots.GGJRootsCharacter|GetMaxLife _asbp_ggjroots_character))
          (goto _label)
          (else
            (bind _output_get (Variables|/Script/GGJRoots.GGJRootsCharacter|SetCurrentLife _asbp_ggjroots_character (+ (Variables|/Script/GGJRoots.GGJRootsCharacter|GetCurrentLife _asbp_ggjroots_character) 1)))
            (bind _asroot_hud (Utilities|Casting|CastToRootHUD (HUD|GetHUD (Pawn|GetLocalViewingPlayerController _asbp_ggjroots_character))))
            (Utilities|IsValid _asroot_hud
              (:Is%20Valid
                (Default|InitialiseLife (Variables|/Game/UI/HUD/HUD.HUD_C|GetWBP_LifeCounter (Variables|/Game/UI/HUD/RootHUD.RootHUD_C|GetHUD%20UI _asroot_hud)))
                (Actor|DestroyActor)))))))))

(event EventBeginPlay)

(event Collision|EventActorBeginOverlap
  (params (OtherActor :type Actor%20Object%20Reference)))

(event EventTick
  (params (DeltaSeconds :type Float%20%28single-precision%29)))

(fn ConstructionScript)