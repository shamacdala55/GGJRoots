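; Enemy stinger projectile that damages the player character on contact.
; When its sphere overlaps a BP_GGJRootsCharacter, it removes one point of CurrentLife, prints the new value and destroys itself.
; It then gets the viewing player's RootHUD and re-initialises the life counter widget so the display reflects the hit.
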(event OnComponentBeginOverlap(Sphere)
  (params (OverlappedComponent :type Primitive%20Component%20Object%20Reference) (OtherActor :type Actor%20Object%20Reference) (OtherComp :type Primitive%20Component%20Object%20Reference) (OtherBodyIndex :type Integer) (bFromSweep :type Boolean) (SweepResult :type Hit%20Result%20Structure%20%28by%20ref%29))
  (bind _asbp_ggjroots_character (Utilities|Casting|CastToBP_GGJRootsCharacter OtherActor))
  (bind _output_get (Variables|/Script/GGJRoots.GGJRootsCharacter|SetCurrentLife _asbp_ggjroots_character (- (Variables|/Script/GGJRoots.GGJRootsCharacter|GetCurrentLife _asbp_ggjroots_character) 1)))
  (Development|PrintString (Utilities|String|ToString(Integer) _output_get))
  (Actor|DestroyActor)
  (bind _asroot_hud (Utilities|Casting|CastToRootHUD (HUD|GetHUD (Pawn|GetLocalViewingPlayerController _asbp_ggjroots_character))))
  (Utilities|IsValid _asroot_hud
    (:Is%20Valid
      (Default|InitialiseLife (Variables|/Game/UI/HUD/HUD.HUD_C|GetWBP_LifeCounter (Variables|/Game/UI/HUD/RootHUD.RootHUD_C|GetHUD%20UI _asroot_hud))))))

(event EventBeginPlay
  (|CallParentFunction) ; This node is disabled and will not be called.\nDrag off pins to build functionality.
)

(event Collision|EventActorBeginOverlap
  (params (OtherActor :type Actor%20Object%20Reference))
  (|CallParentFunction OtherActor) ; This node is disabled and will not be called.\nDrag off pins to build functionality.
)

(event EventTick
  (params (DeltaSeconds :type Float%20%28single-precision%29))
  (|CallParentFunction DeltaSeconds) ; This node is disabled and will not be called.\nDrag off pins to build functionality.
)

(fn ConstructionScript
  (|CallParentFunction))