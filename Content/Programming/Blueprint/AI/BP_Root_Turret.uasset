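; Root turret enemy that turns toward the player character and shoots root projectiles at it.
; PawnSensing sightings that cast to BP_GGJRootsCharacter snap the whole actor's rotation to face the character.
; The same event starts a short Delay, then spawns BP_Projectile_Root at the Turret component's transform.
; Delay ignores retriggers while pending, so it also throttles the fire rate during repeated sightings.
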(event OnSeePawn(PawnSensing)
  (params (Pawn :type Pawn%20Object%20Reference))
  (bind _asbp_ggjroots_character (Utilities|Casting|CastToBP_GGJRootsCharacter Pawn))
  (Utilities|FlowControl|Sequence
    (:then_0
      (Transformation|SetActorRotation (Math|Rotator|FindLookatRotation (Transformation|GetActorLocation) (Transformation|GetActorLocation _asbp_ggjroots_character))))
    (:then_1
      (Utilities|FlowControl|Delay 1.0)
      (Game|SpawnActorfromClass "/Game/Programming/Blueprint/AI/BP_Projectile_Root.BP_Projectile_Root_C" (Transformation|GetWorldTransform (Variables|Default|GetTurret)) "Undefined" 0 0))))

(event EventBeginPlay
  (|CallParentFunction) ; This node is disabled and will not be called.\nDrag off pins to build functionality.
)

(event Collision|EventActorBeginOverlap
  (params (OtherActor :type Actor%20Object%20Reference))
  (|CallParentFunction OtherActor) ; This node is disabled and will not be called.\nDrag off pins to build functionality.
)

(event EventTick
  (params (DeltaSeconds :type Float%20%28single-precision%29))
  (|CallParentFunction DeltaSeconds) ; This node is disabled and will not be called.\nDrag off pins to build functionality.
)

(fn ConstructionScript
  (|CallParentFunction))