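; Base projectile actor that hurts and knocks back the player character (BP_GGJRootsCharacter) on contact.
; Its Sphere's hit and begin-overlap events share one path, which ignores any actor that is not that character.
; That path applies fixed damage, launches the character along the projectile's velocity plus an upward boost, and directly decrements CurrentLife.
; It then reinitialises the character's life counter widget to refresh the display.
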(event OnComponentHit(Sphere)
  (params (HitComponent :type Primitive%20Component%20Object%20Reference) (OtherActor :type Actor%20Object%20Reference) (OtherComp :type Primitive%20Component%20Object%20Reference) (NormalImpulse :type Vector :default "0, 0, 0") (Hit :type Hit%20Result%20Structure%20%28by%20ref%29))
  (bind _asbp_ggjroots_character (Utilities|Casting|CastToBP_GGJRootsCharacter (stale OnComponentBeginOverlap(Sphere) OtherActor)))
  (Game|Damage|ApplyDamage _asbp_ggjroots_character 3e+01 0 0)
  (Character|LaunchCharacter _asbp_ggjroots_character (+ (Transformation|GetVelocity) "0.000000,0.000000,200.000000") false false)
  (Utilities|IsValid _asbp_ggjroots_character
    (:Is%20Valid
      (Variables|/Script/GGJRoots.GGJRootsCharacter|SetCurrentLife _asbp_ggjroots_character (- (Variables|/Script/GGJRoots.GGJRootsCharacter|GetCurrentLife _asbp_ggjroots_character) 1))
      (Utilities|IsValid (Variables|/Game/Programming/Blueprint/Player/BP_GGJRootsCharacter.BP_GGJRootsCharacter_C|GetWBP%20Life%20Counter _asbp_ggjroots_character)
        (:Is%20Valid
          (Default|InitialiseLife (Variables|/Game/Programming/Blueprint/Player/BP_GGJRootsCharacter.BP_GGJRootsCharacter_C|GetWBP%20Life%20Counter _asbp_ggjroots_character)))))))

(event OnComponentBeginOverlap(Sphere)
  (params (OverlappedComponent :type Primitive%20Component%20Object%20Reference) (OtherActor :type Actor%20Object%20Reference) (OtherComp :type Primitive%20Component%20Object%20Reference) (OtherBodyIndex :type Integer) (bFromSweep :type Boolean) (SweepResult :type Hit%20Result%20Structure%20%28by%20ref%29))
  (bind _asbp_ggjroots_character (Utilities|Casting|CastToBP_GGJRootsCharacter OtherActor))
  (Game|Damage|ApplyDamage _asbp_ggjroots_character 3e+01 0 0)
  (Character|LaunchCharacter _asbp_ggjroots_character (+ (Transformation|GetVelocity) "0.000000,0.000000,200.000000") false false)
  (Utilities|IsValid _asbp_ggjroots_character
    (:Is%20Valid
      (Variables|/Script/GGJRoots.GGJRootsCharacter|SetCurrentLife _asbp_ggjroots_character (- (Variables|/Script/GGJRoots.GGJRootsCharacter|GetCurrentLife _asbp_ggjroots_character) 1))
      (Utilities|IsValid (Variables|/Game/Programming/Blueprint/Player/BP_GGJRootsCharacter.BP_GGJRootsCharacter_C|GetWBP%20Life%20Counter _asbp_ggjroots_character)
        (:Is%20Valid
          (Default|InitialiseLife (Variables|/Game/Programming/Blueprint/Player/BP_GGJRootsCharacter.BP_GGJRootsCharacter_C|GetWBP%20Life%20Counter _asbp_ggjroots_character)))))))

(event EventBeginPlay)

(event Collision|EventActorBeginOverlap
  (params (OtherActor :type Actor%20Object%20Reference)))

(event EventTick
  (params (DeltaSeconds :type Float%20%28single-precision%29)))

(fn ConstructionScript)