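; BP_RootPlayerController is the player controller that chooses between gameplay input and the main menu based on the current level.
; On BeginPlay in MainLevel it sets game-only input and hides the cursor.
; In any other level it creates and shows the MainMenu widget with UI-only input and a visible cursor.
; It binds the StartGame button's press to remove the menu, without restoring input mode or cursor.
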(event Custom|OnPressed_Event
  (Widget|RemovefromParent (stale EventBeginPlay _returnvalue_3)))

(event EventBeginPlay
  (bind _returnvalue (Game|GetPlayerController 0))
  (bind _returnvalue_2 (Game|GetCurrentLevelName true))
  (if (Utilities|Enum|Equal(Enum) _returnvalue_2 "MainLevel")
    (Input|SetInputModeGameOnly _returnvalue false)
    (Variables|/Script/Engine.PlayerController|SetbShowMouseCursor _returnvalue false)
    (else
      (bind _returnvalue_3 (UserInterface|CreateWidget "/Game/UI/MainMenu/MainMenu.MainMenu_C"))
      (Variables|/Script/Engine.PlayerController|SetbShowMouseCursor _returnvalue true)
      (Input|SetInputModeUIOnly _returnvalue _returnvalue_3 "DoNotLock" false)
      (UserInterface|Viewport|AddtoViewport _returnvalue_3 0)
      (EventDispatchers|AssignOnPressed (Variables|/Game/UI/MainMenu/MainMenu.MainMenu_C|GetStartGame (Variables|Default|GetMain%20Menu)) (delegate Custom|OnPressed_Event)))))

(event EventTick
  (params (DeltaSeconds :type Float%20%28single-precision%29)))

(fn ConstructionScript)