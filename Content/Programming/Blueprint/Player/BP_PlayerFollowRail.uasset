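; Spline rail actor that constrains the player character to its path between start and end triggers.
; Overlapping StartBox snaps the character onto the spline and passes it a rail reference; EndBox or Endpoint overlap clears both.
; While active, Tick sweeps the capsule to the closest spline X/Y, leaving Z free.
; The construction script builds spline mesh segments and adds Endpoint meshes at the last point, one per segment.
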(event OnComponentBeginOverlap(StartBox)
  (params (OverlappedComponent :type Primitive%20Component%20Object%20Reference) (OtherActor :type Actor%20Object%20Reference) (OtherComp :type Primitive%20Component%20Object%20Reference) (OtherBodyIndex :type Integer) (bFromSweep :type Boolean) (SweepResult :type Hit%20Result%20Structure%20%28by%20ref%29))
  (bind _asbp_ggjroots_character (Utilities|Casting|CastToBP_GGJRootsCharacter OtherActor))
  (bind _output_get (Variables|Default|SetAs%20BP%20GGJRoots%20Character _asbp_ggjroots_character))
  (Utilities|IsValid _output_get
    (:Is%20Valid
      (CallFunction|BeginSpline))))

(event OnComponentBeginOverlap(EndBox)
  (params (OverlappedComponent :type Primitive%20Component%20Object%20Reference) (OtherActor :type Actor%20Object%20Reference) (OtherComp :type Primitive%20Component%20Object%20Reference) (OtherBodyIndex :type Integer) (bFromSweep :type Boolean) (SweepResult :type Hit%20Result%20Structure%20%28by%20ref%29))
  (bind _asbp_ggjroots_character (Utilities|Casting|CastToBP_GGJRootsCharacter (stale OnComponentBeginOverlap(Endpoint) OtherActor)))
  (Utilities|IsValid _asbp_ggjroots_character
    (:Is%20Valid
      (CallFunction|EndSpline))))

(event OnComponentBeginOverlap(Endpoint)
  (params (OverlappedComponent :type Primitive%20Component%20Object%20Reference) (OtherActor :type Actor%20Object%20Reference) (OtherComp :type Primitive%20Component%20Object%20Reference) (OtherBodyIndex :type Integer) (bFromSweep :type Boolean) (SweepResult :type Hit%20Result%20Structure%20%28by%20ref%29))
  (bind _asbp_ggjroots_character (Utilities|Casting|CastToBP_GGJRootsCharacter OtherActor))
  (Utilities|IsValid _asbp_ggjroots_character
    (:Is%20Valid
      (CallFunction|EndSpline))))

(event Custom|BeginSpline
  (bind _as_bp_ggjroots_character (Variables|Default|GetAs%20BP%20GGJRoots%20Character))
  (bind _capsulecomponent (Variables|/Script/Engine.Character|GetCapsuleComponent _as_bp_ggjroots_character))
  (Variables|/Game/Programming/Blueprint/Player/BP_GGJRootsCharacter.BP_GGJRootsCharacter_C|SetInSpline _as_bp_ggjroots_character true)
  (Variables|/Game/Programming/Blueprint/Player/BP_GGJRootsCharacter.BP_GGJRootsCharacter_C|SetSplineReference _as_bp_ggjroots_character self)
  (Transformation|SetWorldLocation _capsulecomponent (Spline|FindLocationClosesttoWorldLocation (Variables|Default|GetSpline) (Transformation|GetWorldLocation _capsulecomponent) "World") false false)
  (Variables|Default|SetSplineActive true)
  (Pawn|Input|AddMovementInput (Variables|/Script/Engine.Actor|GetInstigator (Variables|Default|GetAs%20BP%20GGJRoots%20Character)) "0, 0, 0" 1.0 false))

(event Custom|EndSpline
  (bind _as_bp_ggjroots_character (Variables|Default|GetAs%20BP%20GGJRoots%20Character))
  (Variables|/Game/Programming/Blueprint/Player/BP_GGJRootsCharacter.BP_GGJRootsCharacter_C|SetInSpline _as_bp_ggjroots_character false)
  (Variables|/Game/Programming/Blueprint/Player/BP_GGJRootsCharacter.BP_GGJRootsCharacter_C|SetSplineReference _as_bp_ggjroots_character 0)
  (Variables|Default|SetSplineActive false))

(event EventBeginPlay)

(event Collision|EventActorBeginOverlap
  (params (OtherActor :type Actor%20Object%20Reference)))

(event EventTick
  (params (DeltaSeconds :type Float%20%28single-precision%29))
  (bind _spline (Variables|Default|GetSpline))
  (bind _as_bp_ggjroots_character (Variables|Default|GetAs%20BP%20GGJRoots%20Character))
  (bind _capsulecomponent (Variables|/Script/Engine.Character|GetCapsuleComponent _as_bp_ggjroots_character))
  (bind _returnvalue (Transformation|GetWorldLocation _capsulecomponent))
  (bind _returnvalue_2 (Spline|FindLocationClosesttoWorldLocation _spline _returnvalue "World"))
  (if (Variables|Default|GetSplineActive)
    (Transformation|SetWorldLocation _capsulecomponent (Math|Vector|MakeVector (.x _returnvalue_2) (.y _returnvalue_2) (.Z (Math|Vector|BreakVector _returnvalue))) true false)))

(fn ConstructionScript
  (bind _spline (Variables|Default|GetSpline))
  (bind _spline_2 (Variables|Default|GetSpline))
  (bind _returnvalue (Spline|GetNumberOfSplinePoints _spline))
  (for _index (range 0 (- _returnvalue 2))
    (bind _output_get (Variables|Default|SetIndex _index))
    (bind _returnvalue_2 (AddComponent|AddSplineMeshComponent false))
    (SplineMesh|SetForwardAxis _returnvalue_2 "X" true)
    (Collision|SetCollisionEnabled _returnvalue_2 "QueryAndProbe")
    (SplineMesh|SetStartandEnd _returnvalue_2 (Spline|GetLocationatSplinePoint _spline_2 _output_get "Local") (Spline|GetTangentatSplinePoint _spline_2 _output_get "Local") (Spline|GetLocationatSplinePoint _spline_2 (+ _output_get 1) "Local") (Spline|GetTangentatSplinePoint _spline_2 (+ _output_get 1) "Local") true :!class /Script/Engine.SplineMeshComponent)
    (bind _returnvalue_3 (AddComponent|AddStaticMeshComponent false (Math|Transform|MakeTransform (Spline|GetLocationatSplinePoint _spline_2 (- _returnvalue 1) "Local") "0, 0, 0" "0.500000,0.500000,0.500000")))
    (Variables|Default|SetEndpoint _returnvalue_3)))