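; BP_RootGameModeBase is a game mode that sets up the HUD, plays a game-start sound and keeps a running timer.
; On BeginPlay it creates the HUD widget, adds it to the viewport, then increments Timer through a self-looping one-second Delay instead of Tick.
; The Construction Script also increments Timer once and prints its value.
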(event EventBeginPlay
  (bind _returnvalue (UserInterface|CreateWidget "/Game/UI/HUD/HUD.HUD_C" 0 0))
  (UserInterface|Viewport|AddtoViewport _returnvalue 0)
  (Audio|PlaySound2D "/Game/Music/SoundEffect/Game_Start_2.Game_Start_2" 1.0 1.0 0.0 0 0)
  (Utilities|FlowControl|Delay 1.0 :!label _label)
  (bind _result (Math|Float|IncrementFloat (Variables|Default|GetTimer))
    (:%20%20
      (Variables|Default|SetTimer _result)
      (goto _label))))

(event EventTick
  (params (DeltaSeconds :type Float%20%28single-precision%29)))

(fn ConstructionScript
  (bind _result (Math|Float|IncrementFloat (Variables|Default|GetTimer))
    (:%20%20
      (bind _output_get (Variables|Default|SetTimer _result))
      (Development|PrintString (Utilities|String|ToString(Float) _output_get)))))